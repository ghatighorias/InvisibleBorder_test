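; Base windshield wiper actor that performs one up-and-back sweep each time its Wipe event fires.
; Wipe starts RotatingMovement around the Pivot component, and Tick runs an Up/Down/Stop state machine that reverses the rate at the top and halts at the bottom.
; Side-aware checks detect the top from the forward vector against MaxRotationAngle and the bottom from pitch crossing zero.
; WipingStarted fires at the top reversal, WipingCompleted at the bottom.
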(event Custom|Wipe_Event
  (bind _rotatingmovement (Variables|Default|GetRotatingMovement))
  (if (Utilities|Enum|Equal(Enum) (Variables|MaxRotationAngle|Getdirection) "NewEnumerator2")
    (Variables|MaxRotationAngle|Setdirection "NewEnumerator0")
    (Variables|/Script/Engine.RotatingMovementComponent|SetPivotTranslation _rotatingmovement (Variables|/Script/Engine.SceneComponent|GetRelativeLocation (Variables|Default|GetPivot)))
    (Components|Activation|ToggleActive _rotatingmovement)
    (Variables|/Script/Engine.RotatingMovementComponent|SetRotationRate _rotatingmovement (Variables|MaxRotationAngle|GetMovement_Rate))))

(event EventBeginPlay
  (EventDispatchers|BindEventtoWipe (delegate Custom|Wipe_Event)))

(event EventTick
  (params (DeltaSeconds :type Float%20%28single-precision%29))
  (bind _wiendshield_wiper_side (Variables|MaxRotationAngle|GetWiendshield%20Wiper%20Side))
  (bind _rotatingmovement (Variables|Default|GetRotatingMovement))
  (switch Utilities|FlowControl|Switch|SwitchonWipe_Direction (Variables|MaxRotationAngle|Getdirection)
    (:NewEnumerator0
      (Utilities|ReachedtheTop _wiendshield_wiper_side
        (:Reached
          (Variables|MaxRotationAngle|Setdirection "NewEnumerator1")
          (Variables|/Script/Engine.RotatingMovementComponent|SetRotationRate _rotatingmovement (* (Variables|MaxRotationAngle|GetMovement_Rate) -1))
          (Default|CallWipingStarted))))
    (:NewEnumerator1
      (Utilities|ReachedBottom _wiendshield_wiper_side
        (:Reached
          (Variables|MaxRotationAngle|Setdirection "NewEnumerator2")
          (Components|Activation|ToggleActive _rotatingmovement)
          (Default|CallWipingCompleted))))))

(fn ConstructionScript)