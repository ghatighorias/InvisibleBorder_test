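; DepthMaskCheck is a sample test actor that drives a DepthMask object to paint aging impact marks onto a static mesh's material.
; On BeginPlay it initializes the mask texture with a four-channel impact ratio and starts a looping timer that ages the canvas.
; Each bound impact event rebuilds an elongated circle brush, rotates it by the impact angle and stamps it at the position.
; Tick updates the texture and feeds it to the construction-script dynamic material.
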(event Custom|Impact%20in%20position_Event
  (params (Position :type Vector%202D%20Structure) (angle :type Float%20%28single-precision%29) (pivot :type Vector%202D%20Structure))
  (bind (_x _y) (Math|Vector2D|BreakVector2D Position))
  (bind _mydepthmask (Variables|Default|GetMyDepthMask))
  (Class|MyDepthMaskComponent|CreateCircleBrush _mydepthmask 141 1.0 8e+01)
  (Class|MyDepthMaskComponent|RotateBrush _mydepthmask (* -1 angle) (Utilities|Struct|MakeIntPoint 141 141))
  (Class|MyDepthMaskComponent|ReSetBrush _mydepthmask)
  (Class|MyDepthMaskComponent|ImpactinPosition _mydepthmask (Utilities|Struct|MakeIntPoint (Math|Float|Truncate _x) (Math|Float|Truncate _y))))

(event Custom|Age%20the%20canvas_Event
  (Class|MyDepthMaskComponent|Age (Variables|Default|GetMyDepthMask)))

(event EventBeginPlay
  (bind _mydepthmask (Variables|Default|GetMyDepthMask))
  (bind _canvas_size (Variables|DepthMaskProperties|GetCanvas%20Size))
  (bind (_x _y) (Math|Vector2D|BreakVector2D _canvas_size))
  (Class|MyDepthMaskComponent|CreateCircleBrush _mydepthmask 121 1.0 12.0)
  (Class|MyDepthMaskComponent|RotateBrush _mydepthmask 15.0 (Utilities|Struct|MakeIntPoint 60 60))
  (bind _texture (Class|MyDepthMaskComponent|Initialize _mydepthmask (Utilities|Struct|MakeIntPoint (Math|Float|Truncate _x) (Math|Float|Truncate _y)) (Variables|DepthMaskProperties|GetAging%20Step) (Utilities|Struct|MakeFourChannelImpactRatio 3 1 1) (Variables|DepthMaskProperties|GetImpactRatio) (Variables|DepthMaskProperties|GetImage%20Compression)))
  (Variables|Default|SetDepthMaskTexture _texture)
  (EventDispatchers|BindEventtoImpactinPosition (delegate Custom|Impact%20in%20position_Event))
  (Utilities|Time|SetTimerbyEvent (delegate Custom|Age%20the%20canvas_Event) 0.3 true))

(event EventTick
  (params (DeltaSeconds :type Float%20%28single-precision%29))
  (Class|MyDepthMaskComponent|UpdateMaskTexture (Variables|Default|GetMyDepthMask))
  (Rendering|Material|SetTextureParameterValue (Variables|Default|GetDYM) (Variables|DepthMaskProperties|GetMaterialParameterName) (Variables|Default|GetDepthMaskTexture)))

(fn ConstructionScript
  (bind _returnvalue (Rendering|Material|CreateDynamicMaterialInstance (Variables|Default|GetMaterial) :!class /Script/Engine.KismetMaterialLibrary))
  (bind _output_get (Variables|Default|SetDYM _returnvalue))
  (Rendering|Material|SetMaterial (Variables|Default|GetStaticMesh) 0 _output_get))