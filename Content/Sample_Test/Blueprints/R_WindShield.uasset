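; R_WindShield is a windshield wiper actor that sweeps up and back down once each time its Wipe event fires.
; Wipe starts a RotatingMovement component around the Pivot component's location, ignoring requests while a sweep is running.
; Tick compares actor pitch to the maximum angle and to zero, reversing, then stopping the rotation.
; It signals wiping started at the top turnaround and wiping completed at the bottom.
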(event Custom|Wipe_Event
  (bind _rotatingmovement (Variables|Default|GetRotatingMovement))
  (if (Utilities|Enum|Equal(Enum) (Variables|Default|Getdirection) "NewEnumerator2")
    (Variables|Default|Setdirection "NewEnumerator0")
    (Variables|/Script/Engine.RotatingMovementComponent|SetPivotTranslation _rotatingmovement (Variables|/Script/Engine.SceneComponent|GetRelativeLocation (Variables|Default|GetPivot)))
    (Components|Activation|ToggleActive _rotatingmovement)
    (Variables|/Script/Engine.RotatingMovementComponent|SetRotationRate _rotatingmovement (Variables|WindshieldSettings|GetMovement_Rate))))

(event EventBeginPlay
  (EventDispatchers|BindEventtoWipe (delegate Custom|Wipe_Event)))

(event EventTick
  (params (DeltaSeconds :type Float%20%28single-precision%29))
  (bind _rotatingmovement (Variables|Default|GetRotatingMovement))
  (switch Utilities|FlowControl|Switch|SwitchonWipe_Direction (Variables|Default|Getdirection)
    (:NewEnumerator0
      (Utilities|ReachedtheTop
        (:Reached
          (Variables|Default|Setdirection "NewEnumerator1")
          (Variables|/Script/Engine.RotatingMovementComponent|SetRotationRate _rotatingmovement (* (Variables|WindshieldSettings|GetMovement_Rate) -1))
          (Default|CallWipingStarted))
        (:Not%20Reached
          (Development|PrintString (Utilities|String|ToString(Rotator) (Transformation|GetActorRotation self))))))
    (:NewEnumerator1
      (Utilities|ReachedBottom
        (:Reached
          (Variables|Default|Setdirection "NewEnumerator2")
          (Components|Activation|ToggleActive _rotatingmovement)
          (Default|CallWipingCompleted))))))

(fn ConstructionScript)