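; Car Blueprint that runs two windshield wipers and stamps their wiped area into a DepthMaskCheck mask actor.
; A bound wipe event starts both child-actor wipers and their sound, raising per-side flags that completion callbacks clear.
; While flagged, Tick converts each wiper's impact-center Y/Z location into mask coordinates and stamps it at the blade's pitch.
; Right-wiper completion also changes the mask's impact channel; an immediate-wipe event stamps both sides once.
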(event Custom|WipeWindow_Event
  (bind _windshield_sound (Variables|Default|GetWindshield_sound))
  (bind _aswindshield_base (Utilities|Casting|CastTowindshield_base (Variables|/Script/Engine.ChildActorComponent|GetChildActor (Variables|Default|GetLeft_WindshieldWiper))))
  (bind _aswindshield_base_2 (Utilities|Casting|CastTowindshield_base (Variables|/Script/Engine.ChildActorComponent|GetChildActor (Variables|Default|GetRight_WindshieldWiper))))
  (Variables|Default|SetL_WindShield_is_cleaning true)
  (Default|WipeEvent _aswindshield_base)
  (Variables|Default|SetR_WindShield_is_cleaning true)
  (Default|WipeEvent _aswindshield_base_2)
  ;[1 1 1] Play the sound for the windshield
  (if (not (Audio|Components|Audio|IsPlaying _windshield_sound))
    (Audio|Components|Audio|Play _windshield_sound 0.0)))

(event Custom|immediateWipe_Event
  (Utilities|FlowControl|Sequence
    (:then_0
      (bind (_asdepth_mask_check _impact_position _pitch) (Utilities|CalculatethePointOfImpact (Variables|Default|GetRight_WindshieldWiper)))
      (Default|ImpactinPositionEvent _asdepth_mask_check _impact_position (+ _pitch 5.0) "(X=101.000000,Y=101.000000)"))
    (:then_1
      (bind (_asdepth_mask_check_2 _impact_position_2 _pitch_2) (Utilities|CalculatethePointOfImpact (Variables|Default|GetLeft_WindshieldWiper)))
      (Default|ImpactinPositionEvent _asdepth_mask_check_2 _impact_position_2 (+ _pitch_2 5.0) "(X=101.000000,Y=101.000000)"))))

(event Custom|L_Winshield_Wipe_completed
  (Variables|Default|SetL_WindShield_is_cleaning false))

(event Custom|R_Windshield_Wipe_completed
  (Variables|Default|SetR_WindShield_is_cleaning false)
  (bind _asdepth_mask_check (Utilities|Casting|CastToDepthMaskCheck (Variables|/Script/Engine.ChildActorComponent|GetChildActor (Variables|Default|GetDynamicImage))))
  (Default|ChangeImpactChannel _asdepth_mask_check))

(event EventBeginPlay
  (EventDispatchers|BindEventtoImmediateWipe (delegate Custom|immediateWipe_Event))
  (EventDispatchers|BindEventtoWipeWindow (delegate Custom|WipeWindow_Event))
  (Utilities|FlowControl|Sequence
    (:then_0
      (bind _aswindshield_base (Utilities|Casting|CastTowindshield_base (Variables|/Script/Engine.ChildActorComponent|GetChildActor (Variables|Default|GetLeft_WindshieldWiper))))
      (EventDispatchers|BindEventtoWipingCompleted _aswindshield_base (delegate Custom|L_Winshield_Wipe_completed)))
    (:then_1
      (bind _aswindshield_base_2 (Utilities|Casting|CastTowindshield_base (Variables|/Script/Engine.ChildActorComponent|GetChildActor (Variables|Default|GetRight_WindshieldWiper))))
      (EventDispatchers|BindEventtoWipingCompleted _aswindshield_base_2 (delegate Custom|R_Windshield_Wipe_completed)))))

(event EventTick
  (params (DeltaSeconds :type Float%20%28single-precision%29))
  (Utilities|FlowControl|Sequence
    (:then_0
      (if (Variables|Default|GetR_WindShield_is_cleaning)
        (bind (_asdepth_mask_check _impact_position _pitch) (Utilities|CalculatethePointOfImpact (Variables|Default|GetRight_WindshieldWiper)))
        (Default|ImpactinPositionEvent _asdepth_mask_check _impact_position (+ _pitch 5.0) "(X=101.000000,Y=101.000000)")))
    (:then_1
      (if (Variables|Default|GetL_WindShield_is_cleaning)
        (bind (_asdepth_mask_check_2 _impact_position_2 _pitch_2) (Utilities|CalculatethePointOfImpact (Variables|Default|GetLeft_WindshieldWiper)))
        (Default|ImpactinPositionEvent _asdepth_mask_check_2 _impact_position_2 (+ _pitch_2 5.0) "(X=101.000000,Y=101.000000)")))))

(fn ConstructionScript)

(fn TranslateImpactCenter
  (params (Impact_Center_Parent :type Actor%20Object%20Reference) (Impact_Center :type Target%20Point%20Object%20Reference) (DepthMask :type Depth%20Mask%20Check%20Object%20Reference))
  (bind _returnvalue (Transformation|GetActorScale3D DepthMask))
  (bind _returnvalue_2 (Transformation|GetActorLocation DepthMask))
  (bind _returnvalue_3 (Transformation|GetActorLocation Impact_Center))
  (bind _mask_size (LocalVariables|Getmask_size))
  (bind _returnvalue_4 (/ _mask_size 2.0))
  (bind (_x _y _z) (Math|Vector|BreakVector _returnvalue_3))
  (bind (_x_2 _y_2 _z_2) (Math|Vector|BreakVector _returnvalue_2))
  (bind (_x_3 _y_3 _z_3) (Math|Vector|BreakVector _returnvalue))
  (bind _returnvalue_5 (- _z_2 _z))
  (bind _returnvalue_6 (- _y_2 _y))
  (bind (_x_4 _y_4) (Math|Vector2D|BreakVector2D _returnvalue_4))
  (bind _returnvalue_7 (/ _returnvalue_6 _y_3))
  (bind _returnvalue_8 (/ _returnvalue_5 _z_3))
  (bind _returnvalue_9 (Math|Vector2D|MakeVector2D _returnvalue_7 _returnvalue_8))
  (bind (_x_5 _y_5) (Math|Vector2D|BreakVector2D _returnvalue_9))
  (return (Math|Vector2D|MakeVector2D (- _x_4 _x_5) (+ _y_4 _y_5))))